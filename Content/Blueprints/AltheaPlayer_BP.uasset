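; AltheaPlayer_BP is the player character for Althea, handling animation state, pause and victory screens, and feedback particles.
; BeginPlay caches the anim Blueprint and creates both widgets hidden; the Pause input toggles the menu, cursor, input mode and look/move lock.
; Tick either runs the timed victory screen and particles, or updates glide and in-air flags and times the particle burst triggered through SetJustReceivedAbility.
; Jump flags a double jump when already falling.
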(event `self.ReceiveBeginPlay`
  ;[1 1 1] Store the animation blueprint instance
  (bind _asalthea_anim_bp (cast `/Game/Models/SK_Althea/AltheaAnim_BP` (`SkeletalMeshComponent.GetAnimInstance` (`self.Mesh`))))
  (set `self.AltheaAnimBP` _asalthea_anim_bp)
  ;[1 1 1] Create Pause Menu
  (bind _returnvalue (`|CreateWidget` "/Game/PauseMenuWidget.PauseMenuWidget_C"))
  (bind _output_get (set `self.PauseMenu` _returnvalue))
  (`UserWidget.AddToViewport` _output_get 0)
  (`Widget.SetVisibility` (`self.PauseMenu`) "Hidden")
  (set `self.IsPauseMenuHidden` true)
  ;[1 1 1] Create Victory Screen
  (bind _returnvalue_2 (`|CreateWidget` "/Game/VictoryScreen.VictoryScreen_C"))
  (bind _output_get_2 (set `self.VictoryScreen` _returnvalue_2))
  (`UserWidget.AddToViewport` _output_get_2 0)
  (`Widget.SetVisibility` _output_get_2 "Hidden")
  (set `self.IsVictoryScreenVisible` false)
  (set `self.VictoryScreenDisplayed` false)
  ;[1 1 1] Initialize JustGotAbility to False and Particles to inactive
  (set `self.bJustReceivedAbility` false)
  (`ActorComponent.Deactivate` (`self.ReceivedAbilityParticles`))
  (`ActorComponent.Deactivate` (`self.VictoryParticles`)))

(event `self.ReceiveTick`
  (params (DeltaSeconds :type "Float (single-precision)"))
  (bind (_returnvalue_x _returnvalue_y _returnvalue_z) (`KismetMathLibrary.BreakVector` (`self.GetVelocity`)))
  (bind _receivedabilityparticles (`self.ReceivedAbilityParticles`))
  ;[1 1 1] If Victorious and if it hasn't already been displayed, enable Victory Particles and set Victory Screen visible
  (if (`self.Victorious`)
    (bind _output_get (set `self.TimeSinceVictorious` (+ DeltaSeconds (`self.TimeSinceVictorious`))))
    (if (> _output_get 7.0)
      (`Widget.SetVisibility` (`self.VictoryScreen`) "Hidden")
      (else
        (`ActorComponent.SetActive` (`self.VictoryParticles`) true false)
        (`Widget.SetVisibility` (`self.VictoryScreen`) "Visible")
        (set `self.VictoryScreenDisplayed` true)))
    (else
      ;[1 1 1] Animation Gliding
      (set `self.isGliding` (<= _returnvalue_z -150.0))
      ;[1 1 1] Animation In Air
      (set `self.IsInAir` (`NavMovementComponent.IsFalling` (`self.CharacterMovement`)))
      ;[1 1 1] Increment the time since an ability was received
      (if (`self.bJustReceivedAbility`)
        (bind _output_get_2 (set `self.TimeSinceAbilityReceived` (+ (`self.TimeSinceAbilityReceived`) DeltaSeconds)))
        ;[1 1 1] If the time since an ability was received is within the limits, enable the particles from displaying
        (if (and (> _output_get_2 1.2) (< _output_get_2 2.5))
          (`ActorComponent.SetActive` _receivedabilityparticles true false)
          (else
            (`ActorComponent.SetActive` _receivedabilityparticles false false)
            ;[1 1 1] If the timer has finished, reset the timer
            (if (> (`self.TimeSinceAbilityReceived`) 2.5)
              (set `self.bJustReceivedAbility` false)
              (set `self.TimeSinceAbilityReceived` 0.0))))))))

(event `InputAction|Pause`
  (params (Key :type "Key Structure"))
  (bind _returnvalue (`GameplayStatics.GetPlayerController` 0))
  (bind _pausemenu (`self.PauseMenu`))
  (:`Pressed`
    ;[1 1 1] Hide the Victory screen
    (`Widget.SetVisibility` (`self.VictoryScreen`) "Hidden")
    (if (`self.IsPauseMenuHidden`)
      ;[1 1 1] Hides or shows menu as well as lock or unlocks movement for player
      (`Widget.SetVisibility` _pausemenu "Visible")
      (set `PlayerController.bShowMouseCursor` true _returnvalue)
      (`Controller.SetIgnoreLookInput` _returnvalue true)
      (`Controller.SetIgnoreMoveInput` _returnvalue true)
      (set `self.IsPauseMenuHidden` false)
      (`WidgetBlueprintLibrary.SetInputMode_GameAndUIEx` _returnvalue null)
      (`KismetSystemLibrary.Delay` 0.2)
      (`Widget.SetKeyboardFocus` (`/Game/PauseMenuWidget.Button` (`self.PauseMenu`)))
      (`Widget.SetKeyboardFocus` (`/Game/PauseMenuWidget.Button_1` (`self.PauseMenu`)))
      (`Widget.SetKeyboardFocus` (`/Game/PauseMenuWidget.Button_2` (`self.PauseMenu`)))
      (`Widget.SetKeyboardFocus` (`/Game/PauseMenuWidget.Button_456` (`self.PauseMenu`)))
      (`Widget.SetKeyboardFocus` (`/Game/PauseMenuWidget.Return` (`self.PauseMenu`)))
      (`Widget.SetKeyboardFocus` (`/Game/PauseMenuWidget.Returns` (`self.PauseMenu`)))
      (`Widget.SetKeyboardFocus` (`/Game/PauseMenuWidget.Resolutions` (`self.PauseMenu`)))
      (`Widget.SetKeyboardFocus` (`/Game/PauseMenuWidget.Visual` (`self.PauseMenu`)))
      (else
        (`Widget.SetVisibility` _pausemenu "Hidden")
        (set `PlayerController.bShowMouseCursor` false _returnvalue)
        (`Controller.SetIgnoreLookInput` _returnvalue false)
        (`Controller.SetIgnoreMoveInput` _returnvalue false)
        (set `self.IsPauseMenuHidden` true)
        (`WidgetBlueprintLibrary.SetInputMode_GameOnly` _returnvalue)))))

(event `InputAction|Jump`
  (params (Key :type "Key Structure"))
  ;[1 1 1] Double Jump animation
  (:`Pressed`
    (`self.Jump`)
    (if (`NavMovementComponent.IsFalling` (`self.CharacterMovement`))
      (set `self.IsDoubleJumping` true))))

(fn `SetJustReceivedAbility`
  (params (value :type Boolean))
  (set `self.bJustReceivedAbility` value))

(fn `UserConstructionScript`)