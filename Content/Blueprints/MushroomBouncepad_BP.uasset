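; Mushroom bouncepad actor that shrinks away when a Medium_BP actor overlaps it; no bounce logic is present.
; On BeginPlay it takes a random uniform scale, and the overlap sets a Shrinking flag.
; While flagged, Tick subtracts a fixed, frame-rate-dependent step from the scale.
; It destroys itself only if the scale vector's length, which cannot be negative, hits exactly zero.
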(event `self.ReceiveBeginPlay`
  (`self.SetActorScale3D` (`KismetMathLibrary.Conv_DoubleToVector` (`KismetMathLibrary.RandomFloatInRange` 2.0 0.5))))

(event `self.ReceiveActorBeginOverlap`
  (params (OtherActor :type "Actor Object Reference"))
  (cast `/Game/Blueprints/Medium_BP` OtherActor)
  (set `self.Shrinking` true))

(event `self.ReceiveTick`
  (params (DeltaSeconds :type "Float (single-precision)"))
  ;[1 1 1] If Shrinking, shrink
  (if (`self.Shrinking`)
    (`self.SetActorScale3D` (- (`self.GetActorScale3D`) 0.1))
    ;[1 1 1] If the mushroom's scale has reached or fell below zero, destroy the actor
    (if (<= (`KismetMathLibrary.VSize` (`self.GetActorScale3D`)) 0.0)
      (`self.K2_DestroyActor`))))

(fn `UserConstructionScript`)