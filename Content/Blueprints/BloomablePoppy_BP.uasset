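; BloomablePoppy_BP is a poppy actor that plays its bloom animation through a GeometryCache when triggered by an overlap.
; BeginPlay slightly randomizes its scale for variety.
; Its CollisionSphere starts the animation for any Medium_BP, or for an AltheaPlayer_BP that has Bloom.
; Random rotation and area or tag filtering remain in the graph as disconnected, unused logic.
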(event `self.ReceiveBeginPlay`
  ;[1 1 1] Slightly Randomize the scale
  (`self.SetActorScale3D` (`KismetMathLibrary.Conv_DoubleToVector` (`KismetMathLibrary.RandomFloatInRange` 1.45 1.55))))

(event `self.CollisionSphere.OnComponentBeginOverlap`
  (params (OverlappedComponent :type "PrimitiveComponent Object Reference") (OtherActor :type "Actor Object Reference") (OtherComp :type "PrimitiveComponent Object Reference") (OtherBodyIndex :type Integer) (bFromSweep :type Boolean) (SweepResult :type "HitResult Structure (by ref)"))
  (bind _asmedium_bp (cast `/Game/Blueprints/Medium_BP` OtherActor)
    (:`then`
      ;[1 1 1] Bloom
      (set `GeometryCacheComponent.bRunning` true (`self.GeometryCache`)))
    (:`CastFailed`
      ;[1 1 1] If the player has Bloom
      (bind _asalthea_player_bp (cast `/Game/Blueprints/AltheaPlayer_BP` OtherActor))
      (bind _returnvalue (`AltheaPlayer.GetHasBloom` _asalthea_player_bp))
      (if _returnvalue
        (set `GeometryCacheComponent.bRunning` true (`self.GeometryCache`))))))

(fn `UserConstructionScript`)