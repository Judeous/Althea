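; Area barrier that opens when a Medium_BP actor tagged "Bloom" and "Area" plus its AreaCode overlaps it.
; Actors also tagged "BloomsEverything" do not trigger it.
; A visible barrier slides along negative relative X on Tick at a random, frame-rate-dependent speed, then destroys itself after a maximum distance.
; The InvisibleWall variant hides its mesh at start and only disables collision when triggered.
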(event `self.ReceiveBeginPlay`
  (if (`self.InvisibleWall`)
    ;[1 1 1] Set visibility to false if the Barrier is supposed to be an invisible wall
    (`SceneComponent.SetVisibility` (`self.StaticMesh`) false false)
    (else
      ;[1 1 1] Generate a random move speed for moving out the way
      (set `self.MoveSpeed` (`KismetMathLibrary.RandomFloatInRange` 5.5 8.0)))))

(event `self.StaticMesh.OnComponentBeginOverlap`
  (params (OverlappedComponent :type "PrimitiveComponent Object Reference") (OtherActor :type "Actor Object Reference") (OtherComp :type "PrimitiveComponent Object Reference") (OtherBodyIndex :type Integer) (bFromSweep :type Boolean) (SweepResult :type "HitResult Structure (by ref)"))
  ;[1 1 1] Construct the Area tag
  (bind _output_get (set `self.SArea` "Area"))
  (bind _asmedium_bp (cast `/Game/Blueprints/Medium_BP` OtherActor))
  ;[1 1 1] Check OtherActor tags
  (if (`self.ActorHasTag` _asmedium_bp "BloomsEverything")
    _
    (elif (and (`self.ActorHasTag` _asmedium_bp "Bloom") (`self.ActorHasTag` _asmedium_bp (`KismetStringLibrary.Conv_StringToName` (`KismetStringLibrary.Concat_StrStr` _output_get (`KismetStringLibrary.Conv_IntToString` (`self.AreaCode`))))))
      (set `self.Moving` true))))

(event `self.ReceiveTick`
  (params (DeltaSeconds :type "Float (single-precision)"))
  (bind _staticmesh (`self.StaticMesh`))
  (bind _relativelocation_x (`KismetMathLibrary.BreakVector` (`SceneComponent.RelativeLocation` _staticmesh)))
  ;[1 1 1] Check whether or not Moving is true
  (if (`self.Moving`)
    ;[1 1 1] If the Barrier is an invisible wall, just disable collisions
    (if (`self.InvisibleWall`)
      (`PrimitiveComponent.SetCollisionEnabled` (`self.StaticMesh`) "NoCollision")
      (set `self.Moving` false)
      (else
        ;[1 1 1] Check if the distance it's moved is the maximum distance
        (if (> (`self.MaxMoveDistance`) (`self.CurrentDistanceMoved`))
          ;[1 1 1] Move
          (`SceneComponent.K2_SetRelativeLocation` _staticmesh (`KismetMathLibrary.MakeVector` (+ _relativelocation_x (* (`self.MoveSpeed`) -1.0))) false false)
          ;[1 1 1] Increment distance moved
          (set `self.CurrentDistanceMoved` (+ (`self.CurrentDistanceMoved`) (`self.MoveSpeed`)))
          (else
            (`self.K2_DestroyActor`)))))))

(fn `UserConstructionScript`)